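; BP_ZombieV1 is a zombie enemy character that repeatedly pathfinds toward the player while playing an attached moan sound, re-issuing the move on success or failure.
; Hits subtract health and play flesh sound and Niagara blood effects at the impact point.
; At zero health it disables movement and collision, stops moaning, flags its animation Blueprint as dead, then after five seconds notifies BP_SpawnerV1 and destroys itself.
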(event Custom|MoveTowardPlayer
  (if (not (Variables|Default|GetIsDead))
    (AI|AIMoveTo self "0, 0, 0" (Variables|Default|GetPlayerCharacter) 5.0 false
      (:OnSuccess
        _)
      (:OnFail
        _))
    (CallFunction|MoveTowardPlayer)))

(event Custom|SelfDestroy
  (Utilities|FlowControl|Delay 5.0)
  (CallFunction|SpawnNewZombie)
  (Actor|DestroyActor))

(event EventHit
  (params (Damage :type Float%20%28double-precision%29) (ImpactLocation :type Vector :default "0, 0, 0"))
  (if (not (Variables|Default|GetIsDead))
    (CallFunction|Hitten Damage ImpactLocation)
    (CallFunction|Death)))

(event EventBeginPlay
  (CallFunction|InitializeVariables)
  (CallFunction|MoveTowardPlayer))

(fn ConstructionScript)

(fn PlayHitFeedback
  (params (Location :type Vector))
  (Audio|PlaySoundatLocation "/Game/Assets/Zombie/FX/Hit/MSS_HitFlesh.MSS_HitFlesh" Location "0, 0, 0" 1.0 1.0 0.0 0 0 0 0)
  (Niagara|SpawnSystematLocation "/Game/Assets/Zombie/FX/Hit/NS_Blood.NS_Blood" Location "0, 0, 0" "1.000000,1.000000,1.000000" true true "AutoRelease"))

(fn Death
  (if (<= (Variables|Default|GetHealth) 0.0)
    (Variables|Default|SetIsDead true)
    (Pawn|Components|CharacterMovement|DisableMovement (Variables|Character|GetCharacterMovement))
    (Collision|SetCollisionEnabled (Variables|Collision|GetCapsuleComponent) "NoCollision")
    (Audio|Components|Audio|Stop (Variables|Default|GetMoanAudio))
    (Variables|/Game/Versions/Version1/ABP_Zombie.ABP_Zombie_C|SetIsDead (Variables|Animation|GetAnimationBlueprint) true)
    (CallFunction|SelfDestroy)))

(fn Hitten
  (params (Damage :type Float%20%28double-precision%29) (ImpactLocation :type Vector))
  (Variables|Default|SetHealth (- (Variables|Default|GetHealth) Damage))
  (CallFunction|PlayHitFeedback ImpactLocation))

(fn InitializeVariables
  (Variables|Default|SetPlayerCharacter (Game|GetPlayerCharacter 0))
  (bind _asabp_zombie (Utilities|Casting|CastToABP_Zombie (Components|SkeletalMesh|GetAnimInstance (Variables|Character|GetMesh))))
  (Variables|Animation|SetAnimationBlueprint _asabp_zombie)
  (bind _returnvalue (Audio|SpawnSoundAttached "/Game/Assets/Zombie/FX/Moan/MSS_Moan.MSS_Moan" (Variables|Collision|GetCapsuleComponent) "None" "0, 0, 0" "0, 0, 0" "KeepRelativeOffset" true 1.0 1.0 0.0 "/Game/Assets/Zombie/FX/SA_Moan.SA_Moan" 0 false))
  (Variables|Default|SetMoanAudio _returnvalue))

(fn SpawnNewZombie
  (bind _returnvalue (Actor|GetActorOfClass "/Game/Versions/Version1/BP_SpawnerV1.BP_SpawnerV1_C"))
  (Default|ZombieDie _returnvalue))