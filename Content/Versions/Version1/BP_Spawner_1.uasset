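; BP_Spawner_1 is a spawner actor that populates its SpawnArea box with BP_Zombie_1 actors, creating NbZombies of them on BeginPlay.
; SpawnZombie places each zombie at the actor location plus a random unit vector flattened to XY and scaled by the box extent.
; Its rotation derives from the Y component of another random vector.
; ChangeNbZombies spawns the difference when given a higher count and never removes zombies.
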(event EventBeginPlay
  (for _index (range 0 (- (Variables|Parameters|GetNbZombies) 1))
    (CallFunction|SpawnZombie)))

(fn ConstructionScript)

(fn GetRandomSpawnTransform
  (return (Math|Transform|MakeTransform (+ (Transformation|GetActorLocation) (* (Components|Box|GetScaledBoxExtent (Variables|Default|GetSpawnArea)) (* (Math|Random|RandomUnitVector) "1.000000,1.000000,0.000000"))) (Math|Conversions|RotationFromXVector (* (Math|Random|RandomUnitVector) "0.000000,360.000000,0.000000")) "1.000000,1.000000,1.000000")))

(fn SpawnZombie
  (Game|SpawnActorfromClass "/Game/Versions/Version1/BP_Zombie_1.BP_Zombie_1_C" (CallFunction|GetRandomSpawnTransform) "Undefined" "MultiplyWithRoot" 0 0))

(fn ChangeNbZombies
  (params (NewNbZombie :type Integer))
  (for _index (range 0 (Utilities|Operators|Subtract NewNbZombie (Variables|Parameters|GetNbZombies) 1))
    (CallFunction|SpawnZombie)
    (Variables|Parameters|SetNbZombies NewNbZombie)))