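; Zombie spawner that keeps a target number of BP_ZombieV1 actors alive inside its SpawnArea box.
; It tops up the population on BeginPlay, when ChangeNbZombies sets a new target, and when ZombieDie lowers the live count.
; Random unit vectors flattened to XY and scaled by the box extent place spawns around the actor.
; The rotation math only yields facings along positive or negative world Y.
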(event EventBeginPlay
  (CallFunction|SpawnZombies))

(fn ConstructionScript)

(fn GetRandomSpawnTransform
  (return (Math|Transform|MakeTransform (+ (Transformation|GetActorLocation) (* (Components|Box|GetScaledBoxExtent (Variables|Default|GetSpawnArea)) (* (Math|Random|RandomUnitVector) "1.000000,1.000000,0.000000"))) (Math|Conversions|RotationFromXVector (* (Math|Random|RandomUnitVector) "0.000000,360.000000,0.000000")) "1.000000,1.000000,1.000000")))

(fn SpawnZombie
  (Math|Integer|IncrementInt (Variables|Parameters|GetActualZombieCount)
    (:%20%20
      (Game|SpawnActorfromClass "/Game/Versions/Version1/BP_ZombieV1.BP_ZombieV1_C" (CallFunction|GetRandomSpawnTransform) "AdjustIfPossibleButAlwaysSpawn" "MultiplyWithRoot" 0 0))))

(fn ChangeNbZombies
  (params (NewNbZombie :type Integer))
  (Variables|Parameters|SetNbZombies NewNbZombie)
  (CallFunction|SpawnZombies))

(fn SpawnZombies
  (while (< (Variables|Parameters|GetActualZombieCount) (Variables|Parameters|GetNbZombies))
    (CallFunction|SpawnZombie)))

(fn ZombieDie
  (Math|Integer|DecrementInt (Variables|Parameters|GetActualZombieCount)
    (:%20%20
      (CallFunction|SpawnZombies))))