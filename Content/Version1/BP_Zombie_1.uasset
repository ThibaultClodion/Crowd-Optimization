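; Zombie enemy character that endlessly chases the player, attacks on reaching them, and dies when its health runs out.
; A recursive AI MoveTo loop triggers the animation Blueprint's attack and waits the returned delay before chasing again.
; Hits subtract health and play flesh sound and blood effects; death disables movement and collision, flags the animation, and destroys the actor later.
; A moan loop re-arms itself with random delays whenever its sound finishes.
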(event Custom|MoveTowardPlayer
  (params (Delay :type Float%20%28double-precision%29))
  (if (not (Variables|Default|GetIsDead))
    (Utilities|FlowControl|Delay Delay)
    (AI|AIMoveTo self "0, 0, 0" (Variables|Default|GetPlayerCharacter) 5.0 false
      (:OnSuccess
        (bind _animationtime (Default|StartAttack (Variables|Animation|GetAnimationBlueprint)))
        (CallFunction|MoveTowardPlayer _animationtime))
      (:OnFail
        (CallFunction|MoveTowardPlayer 0.0)))))

(event Custom|MoanLoop
  (if (not (Variables|Default|GetIsDead))
    (Utilities|FlowControl|Delay (Math|Random|RandomFloatinRange (Variables|Moan|GetMinTimeToMoan) (Variables|Moan|GetMaxTimeToMoan)))
    (bind _returnvalue (Audio|SpawnSoundatLocation (Variables|Moan|GetMoanMetaSound) (Transformation|GetActorLocation) "0, 0, 0" 1.0 1.0 0.0 "/Game/Assets/Zombie/FX/SA_Zombie.SA_Zombie" 0))
    (EventDispatchers|BindEventtoOnAudioFinished _returnvalue (delegate Custom|MoanLoop))))

(event Custom|SelfDestroy
  (Utilities|FlowControl|Delay 3e+01)
  (Actor|DestroyActor))

(event EventHit
  (params (Damage :type Float%20%28double-precision%29) (ImpactLocation :type Vector :default "0, 0, 0"))
  (if (not (Variables|Default|GetIsDead))
    (CallFunction|Hitten Damage ImpactLocation)
    (CallFunction|Death)))

(event EventBeginPlay
  (CallFunction|InitializeVariables)
  (CallFunction|MoveTowardPlayer 0.0)
  (CallFunction|MoanLoop))

(fn ConstructionScript)

(fn PlayHitFeedback
  (params (Location :type Vector))
  (Audio|PlaySoundatLocation "/Game/Assets/Zombie/FX/Hit/MSS_HitFlesh.MSS_HitFlesh" Location "0, 0, 0" 1.0 1.0 0.0 0 0 0 0)
  (Niagara|SpawnSystematLocation "/Game/Assets/Zombie/FX/Hit/NS_Blood.NS_Blood" Location "0, 0, 0" "1.000000,1.000000,1.000000" true true "AutoRelease"))

(fn Death
  (if (<= (Variables|Default|GetHealth) 0.0)
    (Variables|Default|SetIsDead true)
    (Pawn|Components|CharacterMovement|DisableMovement (Variables|Character|GetCharacterMovement))
    (Collision|SetCollisionEnabled (Variables|Collision|GetCapsuleComponent) "NoCollision")
    (Variables|/Game/Version1/ABP_Zombie.ABP_Zombie_C|SetIsDead (Variables|Animation|GetAnimationBlueprint) true)
    (CallFunction|SelfDestroy)))

(fn Hitten
  (params (Damage :type Float%20%28double-precision%29) (ImpactLocation :type Vector))
  (Variables|Default|SetHealth (- (Variables|Default|GetHealth) Damage))
  (CallFunction|PlayHitFeedback ImpactLocation))

(fn InitializeVariables
  (Variables|Default|SetPlayerCharacter (Game|GetPlayerCharacter 0))
  (bind _asabp_zombie (Utilities|Casting|CastToABP_Zombie (Components|SkeletalMesh|GetAnimInstance (Variables|Character|GetMesh))))
  (Variables|Animation|SetAnimationBlueprint _asabp_zombie))