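; BP_Gun is a hitscan gun that fires a line trace and plays shot feedback.
; On BeginPlay it caches the camera manager and adds force feedback and Niagara components, the latter at the mesh's Muzzle socket transform.
; Shoot traces forward from MuzzleLocation with the Pawn profile and sends damage and impact point to the hit actor via HitMessage.
; A separate ShootFeedback event triggers rumble, camera shake, gunshot sound and muzzle flash.
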(event EventBeginPlay
  (CallFunction|InitializeVariables))

(event EventShoot
  (bind _muzzlelocation (Variables|Default|GetMuzzleLocation))
  (bind _returnvalue (Transformation|GetWorldLocation _muzzlelocation))
  (bind _outhit (Class|KismetSystemLibrary|LineTraceSinglebyProfile _returnvalue (+ _returnvalue (* (Math|Vector|GetForwardVector _muzzlelocation) 2.5e+03)) "Pawn" false 0 "None" true))
  (Class|BPIHittable|Hit(Message) (.hitactor _outhit) (Variables|Default|GetDamage) (.impactpoint _outhit)))

(event EventShootFeedback
  (Audio|Components|Audio|Play (Variables|Default|GetForceFeedbackComponent) 0.0)
  (Class|LegacyCameraShake|StartLegacyCameraShake (Variables|Components|GetCameraManager) "/Game/Blueprints/Vibrations/BP_ShootCameraShake.BP_ShootCameraShake_C" 1.0 "CameraLocal" "0, 0, 0")
  (Audio|PlaySoundatLocation "/Game/Assets/Weapons/Rifle/SFX/SFX_AR_15_SingleShot.SFX_AR_15_SingleShot" "0, 0, 0" "0, 0, 0" 1.0 1.0 0.0 0 0 0 0)
  (Niagara|SpawnSystemAttached "/Game/Assets/Weapons/Rifle/MuzzleFlash/Niagara/NS_MuzzleFlash.NS_MuzzleFlash" (Variables|Default|GetNiagaraParticleSystem) "None" "0, 0, 0" "0, 0, 0" "KeepRelativeOffset" false true "AutoRelease"))

(fn ConstructionScript)

(fn InitializeVariables
  (bind _returnvalue (AddComponent|AddForceFeedbackComponent false))
  (Variables|Default|SetForceFeedbackComponent _returnvalue)
  (Variables|Components|SetCameraManager (Game|GetPlayerCameraManager 0))
  (bind _returnvalue_2 (AddComponent|AddNiagaraComponent false (Transformation|GetSocketTransform (Variables|Default|GetGunMesh) "Muzzle" "RTS_Component")))
  (Variables|Default|SetNiagaraParticleSystem _returnvalue_2))